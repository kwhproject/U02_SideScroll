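; Game mode for jump-map stages that runs a countdown timer and decides win or game over.
; BeginPlay creates the timer, result and pause widgets and parses the stage number from the level name.
; Tick uses a Delay to step the countdown, killing the player at zero and showing game over on death.
; A cleared treasure chest halts the countdown; only a new highest stage saves progress and shows the win screen.
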(event EventBeginPlay
  (|CreateTimerWidget)
  (|CreateStageClearWidget)
  (|CreateGameOverWidget)
  (|CreatePauseWidget)
  (Utilities|FlowControl|Sequence
    (:then_0
      (Input|SetInputModeGameOnly (Game|GetPlayerController 0)))
    (:then_1
      (bind _returnvalue (Game|GetCurrentLevelName true))
      (bind _asbp_game_instance (Utilities|Casting|CastToBP_GameInstance (Game|GetGameInstance)))
      (Variables|/Game/Blueprints/Game/BP_GameInstance.BP_GameInstance_C|SetCurrentStage _asbp_game_instance (Math|Conversions|ToInteger(Byte) (Utilities|String|Replace _returnvalue "Stage"))))))

(event EventTick
  (params (DeltaSeconds :type Float%20%28single-precision%29))
  (bind _returnvalue (Game|GetPlayerController 0))
  (bind _stageclearwidget (Variables|Default|GetStageClearWidget))
  (bind _asbp_player (Utilities|Casting|CastToBP_Player (Game|GetPlayerCharacter 0)))
  (if (Variables|/Game/Blueprints/Player/BP_Player.BP_Player_C|GetbDead _asbp_player)
    (CallFunction|PlayerDead)
    (else
      (Utilities|FlowControl|Delay 0.1)
      (Default|UpdateTimer (Variables|Default|GetTimerWidget) (Variables|Default|GetTimer))
      (if (<= (Variables|Default|GetTimer) 0.0)
        (Variables|Default|SetTimer 0.0)
        (CallFunction|PlayerDead)
        (else
          (bind _outactors (Actor|GetAllActorsOfClass "/Game/Blueprints/Objects/BP_TreasureChest_A1.BP_TreasureChest_A1_C"))
          (for _array_element _outactors
            _)
          ;[1 1 1] 스테이지 클리어
          (if (Variables|/Game/Blueprints/Objects/BP_TreasureChest_A1.BP_TreasureChest_A1_C|GetbClear _array_element)
            (bind _asbp_game_instance (Utilities|Casting|CastToBP_GameInstance (Game|GetGameInstance)))
            (if (> (Variables|/Game/Blueprints/Game/BP_GameInstance.BP_GameInstance_C|GetCurrentStage _asbp_game_instance) (Variables|/Game/Blueprints/Game/BP_GameInstance.BP_GameInstance_C|GetClearStage _asbp_game_instance))
              (Variables|/Game/Blueprints/Game/BP_GameInstance.BP_GameInstance_C|SetClearStage _asbp_game_instance (Variables|/Game/Blueprints/Game/BP_GameInstance.BP_GameInstance_C|GetCurrentStage _asbp_game_instance))
              (bind _asbp_game_instance_2 (Utilities|Casting|CastToBP_GameInstance (Game|GetGameInstance)))
              (Default|Save _asbp_game_instance_2)
              (Utilities|FlowControl|Delay 3.0)
              (Widget|SetVisibility (Variables|Default|GetStageClearWidget) "Visible")
              (UserInterface|Animation|PlayAnimation _stageclearwidget (Variables|/Game/Widgets/WB_StageClear.WB_StageClear_C|GetYouWin _stageclearwidget) 0.0 1 "Forward" 1.0 false)
              (Variables|/Script/Engine.PlayerController|SetbShowMouseCursor _returnvalue true)
              (Input|SetInputModeGameandUI _returnvalue 0 "DoNotLock" true))
            (else
              ;[1 1 1] 타이머
              (Variables|Default|SetTimer (- (Variables|Default|GetTimer) 0.1)))))))))

(fn ConstructionScript)

(fn PlayerDead
  (bind _returnvalue (Game|GetPlayerController 0))
  (bind _asbp_player (Utilities|Casting|CastToBP_Player (Game|GetPlayerCharacter 0)))
  (Game|Damage|ApplyDamage _asbp_player 999.0 0 0)
  (if (Variables|/Game/Blueprints/Player/BP_Player.BP_Player_C|GetbDead _asbp_player)
    (Widget|SetVisibility (Variables|Default|GetGameOverWidget) "Visible")
    (Variables|/Script/Engine.PlayerController|SetbShowMouseCursor _returnvalue true)
    (Input|SetInputModeUIOnly _returnvalue 0 "DoNotLock")))

(fn OnRepTimer
  (bind _asbp_game_instance (Utilities|Casting|CastToBP_GameInstance (Game|GetGameInstance)))
  (Default|UpdateTimer (Variables|/Game/Blueprints/Game/BP_GameInstance.BP_GameInstance_C|GetTimerWidget _asbp_game_instance) (Variables|Default|GetTimer)))