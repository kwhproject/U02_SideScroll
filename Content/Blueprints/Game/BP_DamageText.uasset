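; BP_DamageText is a floating damage number actor that shows a damage value and then removes itself.
; On BeginPlay it records its start location and plays a timeline that drives the text's vertical offset and the actor's uniform scale.
; When the timeline finishes, the actor destroys itself.
; SetDamageText converts the passed damage to text for the TextRender component.
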(event EventBeginPlay
  (Variables|Default|SetStartLocation (Transformation|GetActorLocation))
  (bind _output (Timeline|Timeline Play)
    (:Update
      (Transformation|SetWorldLocation (Variables|Default|GetTextRender) (+ (Variables|Default|GetStartLocation) (Math|Vector|MakeVector 0.0 0.0 (.X (Math|Vector|BreakVector _output)))) false false)
      (Transformation|SetActorScale3D (Math|Conversions|ToVector(Float) (.Y (Math|Vector|BreakVector _output)))))
    (:Finished
      (Actor|DestroyActor))))

(fn ConstructionScript)

(fn SetDamageText
  (params (Damage :type Float%20%28single-precision%29))
  (Rendering|Components|TextRender|SetText (Variables|Default|GetTextRender) (Utilities|Text|ToText(Float) Damage "HalfToEven")))