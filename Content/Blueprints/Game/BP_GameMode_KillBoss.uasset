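; Game mode for boss-kill stages, deciding stage clear or game over.
; On BeginPlay it finds the "Boss"-tagged BP_Boss, creates hidden clear, pause and game-over widgets, and derives the stage number from the level name.
; Tick polls the boss: on death it updates and saves GameInstance progress every tick, while a DoOnce damages all non-player Characters and shows the delayed clear screen.
; Otherwise, player death shows game over.
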(event EventBeginPlay
  (|GetBoss
    (:%20
      (|CreateStageClearWidget)
      (|CreatePauseWidget)
      (|CreateGameOverWidget)
      (|SetInputMode)
      (bind _returnvalue (Game|GetCurrentLevelName true))
      (bind _asbp_game_instance (Utilities|Casting|CastToBP_GameInstance (Game|GetGameInstance)))
      (Variables|/Game/Blueprints/Game/BP_GameInstance.BP_GameInstance_C|SetCurrentStage _asbp_game_instance (Math|Conversions|ToInteger(Byte) (Utilities|String|Replace _returnvalue "Stage"))))))

(event EventTick
  (params (DeltaSeconds :type Float%20%28single-precision%29))
  (bind _returnvalue (Game|GetPlayerController 0))
  (bind _returnvalue_2 (Game|GetPlayerController 0))
  (bind _stageclearwidget (Variables|Default|GetStageClearWidget))
  ;[1 1 1] 보스 사망 여부 체크
  (bind _boss (Variables|Default|GetBoss)
    (:then
      (if (Utilities|Enum|Equal(Enum) (Variables|/Game/Blueprints/Boss/BP_Boss.BP_Boss_C|GetBehavior _boss) "NewEnumerator3")
        ;[1 1 1] 스테이지 해금
        (bind _asbp_game_instance (Utilities|Casting|CastToBP_GameInstance (Game|GetGameInstance)))
        (if (> (Variables|/Game/Blueprints/Game/BP_GameInstance.BP_GameInstance_C|GetCurrentStage _asbp_game_instance) (Variables|/Game/Blueprints/Game/BP_GameInstance.BP_GameInstance_C|GetClearStage _asbp_game_instance))
          (Variables|/Game/Blueprints/Game/BP_GameInstance.BP_GameInstance_C|SetClearStage _asbp_game_instance (Variables|/Game/Blueprints/Game/BP_GameInstance.BP_GameInstance_C|GetCurrentStage _asbp_game_instance)))
        (bind _asbp_game_instance_2 (Utilities|Casting|CastToBP_GameInstance (Game|GetGameInstance)))
        (Default|Save _asbp_game_instance_2)
        ;[1 1 1] KillAll
        (Utilities|FlowControl|DoOnce false
          (:Completed
            (bind _outactors (Actor|GetAllActorsOfClass "/Script/Engine.Character"))
            (for _array_element _outactors
              (Utilities|Casting|CastToBP_Player _array_element
                (:CastFailed
                  (Game|Damage|ApplyDamage _array_element 999.0 0 self))))
            ;[1 1 1] 스테이지 클리어 위젯 표시
            (Utilities|FlowControl|Delay 3.0)
            (Widget|SetVisibility (Variables|Default|GetStageClearWidget) "Visible")
            (UserInterface|Animation|PlayAnimation _stageclearwidget (Variables|/Game/Widgets/WB_StageClear.WB_StageClear_C|GetYouWin _stageclearwidget) 0.0 1 "Forward" 1.0 false)
            (Variables|/Script/Engine.PlayerController|SetbShowMouseCursor _returnvalue_2 true)
            (Input|SetInputModeGameandUI _returnvalue_2 0 "DoNotLock" true)))
        (else
          (bind _asbp_player (Utilities|Casting|CastToBP_Player (Game|GetPlayerCharacter 0)))
          (if (Variables|/Game/Blueprints/Player/BP_Player.BP_Player_C|GetbDead _asbp_player)
            (Widget|SetVisibility (Variables|Default|GetGameOverWidget) "Visible")
            (Variables|/Script/Engine.PlayerController|SetbShowMouseCursor _returnvalue true)
            (Input|SetInputModeUIOnly _returnvalue 0 "DoNotLock")))))
    (:else)))

(fn ConstructionScript)