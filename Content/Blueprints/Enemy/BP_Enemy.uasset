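; Melee enemy character that chases the player and attacks with a weapon, driven by a Behavior state machine on Tick using player distance.
; Attack montages pair with events that toggle weapon collision and choose the next behavior; a per-swing actor list prevents repeat hits on "Body"-tagged components.
; Damage triggers knockback, a material flash and floating text, or death and delayed destruction.
; A CurrentHP OnRep function updates the spawned health widget actor.
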(event OnComponentBeginOverlap(WeaponCollision)
  (params (OverlappedComponent :type Primitive%20Component%20Object%20Reference) (OtherActor :type Actor%20Object%20Reference) (OtherComp :type Primitive%20Component%20Object%20Reference) (OtherBodyIndex :type Integer) (bFromSweep :type Boolean) (SweepResult :type Hit%20Result%20Structure%20%28by%20ref%29))
  ;[1 1 1] Weapon Collision Overlapped
  (Variables|Default|SetOtherComp OtherComp)
  (bind _output_get (Variables|Default|SetOtherActor OtherActor))
  (if (!= _output_get self)
    (if (CallFunction|IsOverlappedBody (Variables|Default|GetOtherComp))
      (bind _asbp_player (Utilities|Casting|CastToBP_Player (Variables|Default|GetOtherActor)))
      (if (CallFunction|IsNotMultiHitted)
        (Game|Damage|ApplyDamage _asbp_player (Variables|Default|GetAtk) 0 self)))))

(event Custom|DamageEffect
  ;[1 1 1] Hitted
  (CallFunction|PlayDamageText)
  (Effects|SpawnEmitterAttached "/Game/InfinityBladeEffects/Effects/FX_Mobile/Fire/combat/P_FireBall_Powerup.P_FireBall_Powerup" (Variables|Character|GetMesh) "Head")
  (Rendering|Material|SetVectorParameterValue (Variables|Default|GetDynamicMaterial) "HitColor" "(R=1.000000,G=0.000000,B=0.000000,A=1.000000)" :!class /Script/Engine.MaterialInstanceDynamic)
  (Utilities|FlowControl|Delay 0.1)
  (Rendering|Material|SetVectorParameterValue (Variables|Default|GetDynamicMaterial) "HitColor" "(R=0.000000,G=0.000000,B=0.000000,A=1.000000)" :!class /Script/Engine.MaterialInstanceDynamic))

(event Custom|Attacked
  ;[1 1 1] Attacked
  (CallFunction|NextBehavior))

(event Custom|OnCollision
  ;[1 1 1] On/Off Collision
  (Collision|SetCollisionEnabled (Variables|Default|GetWeaponCollision) "QueryAndPhysics"))

(event Custom|OffCollision
  ;[1 1 1] On/Off Collision
  (Collision|SetCollisionEnabled (Variables|Default|GetWeaponCollision) "NoCollision")
  (Utilities|Array|Clear (Variables|Default|GetHittedActors)))

(event Custom|Hitted
  ;[1 1 1] Hitted
  (CallFunction|NextBehavior))

(event EventBeginPlay
  ;[1 1 1] BeginPlay
  (bind _returnvalue (Rendering|Material|CreateDynamicMaterialInstance "/Game/Characters/Goblin/phong1.phong1" "None" :!class /Script/Engine.KismetMaterialLibrary))
  (bind _output_get (Variables|Default|SetDynamicMaterial _returnvalue))
  (Rendering|Material|SetMaterial (Variables|Character|GetMesh) 1 _output_get)
  (Collision|SetCollisionEnabled (Variables|Default|GetWeaponCollision) "NoCollision")
  (bind _returnvalue_2 (Game|SpawnActorfromClass "/Game/Blueprints/Enemy/BP_EnemyHP.BP_EnemyHP_C" (Math|Transform|MakeTransform (Transformation|GetWorldLocation (Variables|Default|GetHPWidgetSocket))) "Undefined" self 0))
  (Variables|Default|SetHPWidgetActor _returnvalue_2)
  (Variables|Default|SetCurrentHP (Variables|Default|GetMaxHP)))

(event EventTick
  (params (DeltaSeconds :type Float%20%28single-precision%29))
  ;[1 1 1] Tick
  (if (not (CallFunction|IsPlayerDead))
    (|GetPlayerDistance&Direction)
    (switch Utilities|FlowControl|Switch|SwitchonEBehaviorType (Variables|Default|GetBehavior)
      (:NewEnumerator0
        (if (<= (Variables|Default|GetDistanceToPlayer) 5e+02)
          (Variables|Default|SetBehavior "NewEnumerator1")))
      (:NewEnumerator1
        (if (<= (Variables|Default|GetDistanceToPlayer) 1.3e+02)
          (Variables|Default|SetBehavior "NewEnumerator2")
          (Animation|PlayAnimMontage "/Game/Characters/Goblin/Animations/Attack_Montage.Attack_Montage" 1.5 "None")
          (Variables|Default|SetAttacking true)
          (else
            (Pawn|Input|AddMovementInput (Variables|Default|GetDirectionToPlayer) 1.0 false))))
      (:NewEnumerator2
        (if (not (Variables|Default|GetAttacking))
          (if (> (Variables|Default|GetDistanceToPlayer) 1.5e+02)
            (Variables|Default|SetBehavior "NewEnumerator1"))))
      (:NewEnumerator3
        (Utilities|FlowControl|Delay 3.0)
        (Actor|DestroyActor)))))

(event Game|Damage|EventAnyDamage
  (params (Damage :type Float%20%28single-precision%29) (DamageType :type Damage%20Type%20Object%20Reference) (InstigatedBy :type Controller%20Object%20Reference) (DamageCauser :type Actor%20Object%20Reference))
  ;[1 1 1] Hitted
  (Variables|Default|SetDamage Damage)
  (if (Utilities|Enum|NotEqual(Enum) (Variables|Default|GetBehavior) "NewEnumerator3")
    (Variables|Default|SetAttacking false)
    (Collision|SetCollisionEnabled (Variables|Default|GetWeaponCollision) "NoCollision")
    (Audio|PlaySoundatLocation 0 (Transformation|GetActorLocation) "0, 0, 0" 1.0 1.0 0.0 0 0 0)
    (CallFunction|DamageEffect)
    (bind _output_get (Variables|Default|SetCurrentHP (- (Variables|Default|GetCurrentHP) (Variables|Default|GetDamage))))
    (if (<= _output_get 0.0)
      (Variables|Default|SetBehavior "NewEnumerator3")
      (Animation|PlayAnimMontage "/Game/Characters/Goblin/Animations/Falling_Back_Death_Montage.Falling_Back_Death_Montage" 1.0 "None")
      (else
        (Character|LaunchCharacter (* (* (Variables|Default|GetDirectionToPlayer) -1) 500) false false)
        (Variables|Default|SetBehavior "NewEnumerator5")
        (Animation|PlayAnimMontage "/Game/Characters/Goblin/Animations/Sword_And_Shield_Impact_Montage.Sword_And_Shield_Impact_Montage" 1.0 "None")))))

(fn ConstructionScript)

(fn IsPlayerDead
  (bind _asbp_player (Utilities|Casting|CastToBP_Player (Game|GetPlayerCharacter 0)))
  (return (Variables|/Game/Blueprints/Player/BP_Player.BP_Player_C|GetbDead _asbp_player)))

(fn IsOverlappedBody
  (params (OtherComp :type Actor%20Component%20Object%20Reference))
  (bind _componenttags (Variables|/Script/Engine.ActorComponent|GetComponentTags OtherComp))
  (if (> (Utilities|Array|Length _componenttags) 0)
    (return (Utilities|Name|Equal(Name) (Utilities|Array|Get(acopy) _componenttags) "Body"))
    (else
      (return false))))

(fn NextBehavior
  (if (Class|Actor|IsActorTickEnabled)
    (if (not (CallFunction|IsPlayerDead))
      (Variables|Default|SetAttacking false)
      (if (<= (Variables|Default|GetDistanceToPlayer) 1.5e+02)
        (Transformation|SetActorRotation (Math|Conversions|RotationFromXVector (Variables|Default|GetDirectionToPlayer)))
        (Variables|Default|SetBehavior "NewEnumerator2")
        (Animation|PlayAnimMontage "/Game/Characters/Goblin/Animations/Attack_Montage.Attack_Montage" 1.5 "None")
        (Variables|Default|SetAttacking true)
        (else
          (Variables|Default|SetBehavior "NewEnumerator1"))))))

(fn OnRepCurrentHP
  (bind _aswb_enemy_hp (Utilities|Casting|CastToWB_EnemyHP (UserInterface|GetUserWidgetObject (Variables|/Game/Blueprints/Enemy/BP_EnemyHP.BP_EnemyHP_C|GetHPWidgetComp (Variables|Default|GetHPWidgetActor)))))
  (Default|UpdateHealth _aswb_enemy_hp (Variables|Default|GetCurrentHP) (Variables|Default|GetMaxHP)))

(fn PlayDamageText
  (bind _returnvalue (Game|SpawnActorfromClass "/Game/Blueprints/Game/BP_DamageText.BP_DamageText_C" (Math|Transform|MakeTransform (+ (Transformation|GetActorLocation) (Math|Vector|MakeVector -5e+01 0.0 5e+01))) "Undefined" 0 0))
  (Default|SetDamageText _returnvalue (Variables|Default|GetDamage)))

(fn IsNotMultiHitted
  (LocalVariables|SetEverHittedActorNumbers (Utilities|Array|Length (Variables|Default|GetHittedActors)))
  (Utilities|Array|AddUnique (Variables|Default|GetHittedActors) (Variables|Default|GetOtherActor))
  (return (< (LocalVariables|GetEverHittedActorNumbers) (Utilities|Array|Length (Variables|Default|GetHittedActors)))))