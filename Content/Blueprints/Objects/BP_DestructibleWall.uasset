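; BP_DestructibleWall is a wall actor that breaks the first time it takes any damage, with a chance to spawn something in its place.
; A DoOnce gate on AnyDamage disables the Box collision, then randomly either plays the PaladinHit sound or spawns a random entry from RandomActors at the wall's transform.
; After either outcome, the wall destroys itself following a short delay.
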(event Game|Damage|EventAnyDamage
  (params (Damage :type Float%20%28single-precision%29) (DamageType :type Damage%20Type%20Object%20Reference) (InstigatedBy :type Controller%20Object%20Reference) (DamageCauser :type Actor%20Object%20Reference))
  (bind _returnvalue (Math|Random|RandomIntegerinRange 0 3))
  (Utilities|FlowControl|DoOnce false
    (:Completed
      (Collision|SetCollisionEnabled (Variables|Default|GetBox) "NoCollision")
      (if (> _returnvalue 1)
        (Audio|PlaySound2D "/Game/Sounds/PaladinHit.PaladinHit" 1.0 1.0 0.0 0 0)
        (else
          (Game|SpawnActorfromClass (Utilities|Array|Get(acopy) (Variables|Default|GetRandomActors) _returnvalue) (Transformation|GetActorTransform) "Undefined" 0 0)))
      (Utilities|FlowControl|Delay 2.0)
      (Actor|DestroyActor))))

(fn ConstructionScript)