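; BP_Cinematic_Trigger is a placed trigger that plays a Level Sequence cutscene the first time BP_Player overlaps it.
; It keeps its CinematicActors hidden until then, reveals them, and hides and stops ticking every Character and BP_EnemyHP actor while disabling player input and status UI.
; A timer set to the sequence's end time restores gameplay actors, input and boss/player UI, then destroys the cinematic actors.
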(event Custom|OnFinish_Cinematics
  (bind _outactors (Actor|GetAllActorsOfClass "/Script/Engine.Actor"))
  (for _array_element _outactors
    (if (or (Utilities|ClassIsChildOf (Utilities|GetClass _array_element) "/Script/Engine.Character") (Utilities|ClassIsChildOf (Utilities|GetClass _array_element) "/Game/Blueprints/Enemy/BP_EnemyHP.BP_EnemyHP_C"))
      (Rendering|SetActorHiddenInGame _array_element false)
      (Actor|Tick|SetActorTickEnabled _array_element true)))
  (Input|EnableInput (Game|GetPlayerCharacter 0) (Game|GetPlayerController 0))
  (bind _asbp_game_instance (Utilities|Casting|CastToBP_GameInstance (Game|GetGameInstance)))
  (Default|ShowBossStatus _asbp_game_instance true)
  (Default|ShowPlayerStatus _asbp_game_instance true)
  (for _array_element_2 (Variables|Default|GetCinematicActors)
    (Actor|DestroyActor _array_element_2)))

(event EventBeginPlay
  (for _array_element (Variables|Default|GetCinematicActors)
    (Rendering|SetActorHiddenInGame _array_element true)))

(event Collision|EventActorBeginOverlap
  (params (OtherActor :type Actor%20Object%20Reference))
  (Utilities|Casting|CastToBP_Player OtherActor)
  (Utilities|FlowControl|DoOnce false
    (:Completed
      (for _array_element (Variables|Default|GetCinematicActors)
        (Rendering|SetActorHiddenInGame _array_element false))
      (bind _returnvalue (Sequencer|Player|CreateLevelSequencePlayer "/Game/Cinematics/Master.Master"))
      (bind _output_get (Variables|Default|SetSequencePlayer _returnvalue))
      (Utilities|Time|SetTimerbyEvent (delegate Custom|OnFinish_Cinematics) (Class|TimeManagementBlueprintLibrary|ToSeconds(QualifiedFrameTime) (Class|MovieSceneSequencePlayer|GetEndTime _output_get)))
      (Sequencer|Player|Play (Variables|Default|GetSequencePlayer) :!class /Script/MovieScene.MovieSceneSequencePlayer)
      (bind _outactors (Actor|GetAllActorsOfClass "/Script/Engine.Actor"))
      (for _array_element_2 _outactors
        (if (or (Utilities|ClassIsChildOf (Utilities|GetClass _array_element_2) "/Script/Engine.Character") (Utilities|ClassIsChildOf (Utilities|GetClass _array_element_2) "/Game/Blueprints/Enemy/BP_EnemyHP.BP_EnemyHP_C"))
          (Rendering|SetActorHiddenInGame _array_element_2 true)
          (Actor|Tick|SetActorTickEnabled _array_element_2)))
      (Input|DisableInput (Game|GetPlayerCharacter 0) (Game|GetPlayerController 0))
      (bind _asbp_game_instance (Utilities|Casting|CastToBP_GameInstance (Game|GetGameInstance)))
      (Default|ShowBossStatus _asbp_game_instance false)
      (Default|ShowPlayerStatus _asbp_game_instance false))))

(fn ConstructionScript)