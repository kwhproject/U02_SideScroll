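; BP_EntryRock2 is a rock actor that moves back and forth along its own up axis, starting at BeginPlay.
; It stores its start location and an end point offset by Dif along the up vector.
; A timeline lerps the actor between the two points without sweeping.
; Each time the timeline finishes, a FlipFlop switches between Play and Reverse, so the motion loops continuously.
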(event EventBeginPlay
  (bind _returnvalue (Transformation|GetActorLocation))
  (Variables|Default|SetStart _returnvalue)
  (Variables|Default|SetEnd (+ _returnvalue (* (Transformation|GetActorUpVector) (Variables|Default|GetDif))))
  (Utilities|FlowControl|FlipFlop :!label _label
    (:A
      (bind _output (Timeline|타임라인_0 Play)
        (:Update
          (Transformation|SetActorLocation (Math|Vector|Lerp(Vector) (Variables|Default|GetStart) (Variables|Default|GetEnd) _output) false false))
        (:Finished
          (goto _label))))
    (:B
      (Timeline|타임라인_0 Reverse))))

(fn ConstructionScript)