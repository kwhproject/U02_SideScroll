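; BP_Potion is a healing potion object that bobs up and down in the level.
; On BeginPlay, a Timeline lerps its location 50 units along its up vector, and the Finished output re-enters a FlipFlop to alternate play and reverse endlessly.
; IncreaseHP adds Amount to the given player's CurrentHP, clamped between zero and MaxHP, though nothing in this Blueprint calls it.
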(event EventBeginPlay
  (bind _returnvalue (Transformation|GetActorLocation))
  (Variables|Default|SetStart _returnvalue)
  (Variables|Default|SetEnd (+ _returnvalue (* (Transformation|GetActorUpVector) 5e+01)))
  (Utilities|FlowControl|FlipFlop :!label _label
    (:A
      (bind _output (Timeline|Timeline Play)
        (:Update
          (Transformation|SetActorLocation (Math|Vector|Lerp(Vector) (Variables|Default|GetStart) (Variables|Default|GetEnd) _output) false false))
        (:Finished
          (goto _label))))
    (:B
      (Timeline|Timeline Reverse))))

(fn ConstructionScript)

(fn IncreaseHP
  (params (Player :type BP%20Player%20Object%20Reference))
  (Variables|/Game/Blueprints/Player/BP_Player.BP_Player_C|SetCurrentHP Player (Math|Float|Clamp(Float) (+ (Variables|/Game/Blueprints/Player/BP_Player.BP_Player_C|GetCurrentHP Player) (Variables|Default|GetAmount)) 0.0 (Variables|/Game/Blueprints/Player/BP_Player.BP_Player_C|GetMaxHP Player))))