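; BP_Trap is a constantly rotating trap actor that deals repeated damage to Characters overlapping it.
; Tick adds a fixed world rotation each frame, independent of delta time.
; Overlap events add and remove Characters in HittedCharacters, and each Character entering sets a looping TakeDamage timer that is never cleared.
; TakeDamage applies Atk damage to every tracked Character, with the trap as damage causer.
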(event EventTick
  (params (DeltaSeconds :type Float%20%28single-precision%29))
  (Class|Actor|AddActorWorldRotation "0.000000,0.000000,10.000000"))

(event Collision|EventActorBeginOverlap
  (params (OtherActor :type Actor%20Object%20Reference))
  (bind _ascharacter (Utilities|Casting|CastToCharacter OtherActor))
  (Utilities|Array|AddUnique (Variables|Default|GetHittedCharacters) _ascharacter)
  (Utilities|Time|SetTimerbyFunctionName self "TakeDamage" 0.1 true))

(event Collision|EventActorEndOverlap
  (params (OtherActor :type Actor%20Object%20Reference))
  (bind _ascharacter (Utilities|Casting|CastToCharacter OtherActor))
  (Utilities|Array|RemoveItem (Variables|Default|GetHittedCharacters) _ascharacter))

(fn ConstructionScript)

(fn TakeDamage
  (for _array_element (Variables|Default|GetHittedCharacters)
    (Game|Damage|ApplyDamage _array_element (Variables|Default|GetAtk) 0 self)))