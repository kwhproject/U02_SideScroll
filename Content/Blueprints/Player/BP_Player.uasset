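; Player character for a side-view action game, with single-axis movement, jump, timeline-driven dodge roll and three-hit sword combo.
; Attacks and rolls snap facing to the last input, and combos chain through a buffered click.
; Sword overlaps damage tagged components once per swing, while damage flashes a dynamic material and CurrentHP's OnRep updates the HUD.
; Also handles potion pickups, death, the F10 pause menu and debug kill and teleport keys.
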(event OnComponentBeginOverlap(SwordCollision)
  (params (OverlappedComponent :type Primitive%20Component%20Object%20Reference) (OtherActor :type Actor%20Object%20Reference) (OtherComp :type Primitive%20Component%20Object%20Reference) (OtherBodyIndex :type Integer) (bFromSweep :type Boolean) (SweepResult :type Hit%20Result%20Structure%20%28by%20ref%29))
  ;[1 1 1] 무기 충돌 이벤트
  (Variables|Default|SetSweepResult SweepResult)
  (Variables|Default|SetOtherComp OtherComp)
  (bind _output_get (Variables|Default|SetOtherActor OtherActor))
  (if (!= _output_get self)
    (if (CallFunction|IsOverlappedBody (Variables|Default|GetOtherComp))
      (if (CallFunction|IsNotMultiHitted)
        (Game|Damage|ApplyPointDamage (Variables|Default|GetOtherActor) (Variables|Default|GetAtk) (Transformation|GetActorLocation (Variables|Default|GetOtherActor)) (Variables|Default|GetSweepResult) 0 self)
        (Class|PlayerCameraManager|PlayCameraShake (Game|GetPlayerCameraManager 0) "/Game/Blueprints/Camera/BP_HitShake.BP_HitShake_C" 1.0 "CameraLocal" "0, 0, 0")))))

(event OnComponentBeginOverlap(CapsuleComponent)
  (params (OverlappedComponent :type Primitive%20Component%20Object%20Reference) (OtherActor :type Actor%20Object%20Reference) (OtherComp :type Primitive%20Component%20Object%20Reference) (OtherBodyIndex :type Integer) (bFromSweep :type Boolean) (SweepResult :type Hit%20Result%20Structure%20%28by%20ref%29))
  ;[1 1 1] Potion
  (bind _asbp_potion (Utilities|Casting|CastToBP_Potion OtherActor))
  (Default|IncreaseHP _asbp_potion self)
  (Actor|DestroyActor _asbp_potion)
  (Effects|SpawnEmitterAttached "/Game/FXVarietyPack/Particles/P_ky_healAura.P_ky_healAura" (Variables|Character|GetMesh) "" "0, 0, 0" "0, 0, 0" "0.500000,0.500000,1.000000")
  (Audio|PlaySoundatLocation "/Game/Sounds/FairyDrop.FairyDrop" (Transformation|GetActorLocation) "0, 0, 0" 1.0 1.0 0.0 0 0 0))

(event Custom|EndAttack
  ;[1 1 1] 공격
  (Variables|Default|SetbAttacking false)
  (Variables|Default|SetbNextCombo false)
  (Variables|Default|SetComboCount 0)
  (Variables|Default|SetbRolling false))

(event Custom|ChangeHitColor
  ;[1 1 1] Hitted
  (Rendering|Material|SetVectorParameterValue (Variables|Default|GetDynamicMaterial) "Emissive" "(R=1.000000,G=0.000000,B=0.000000,A=1.000000)" :!class /Script/Engine.MaterialInstanceDynamic)
  (Utilities|FlowControl|Delay 0.1)
  (Rendering|Material|SetVectorParameterValue (Variables|Default|GetDynamicMaterial) "Emissive" "(R=0.000000,G=0.000000,B=0.000000,A=1.000000)" :!class /Script/Engine.MaterialInstanceDynamic))

(event Custom|NextCombo
  ;[1 1 1] 공격
  (if (Variables|Default|GetbRolling)
    (CallFunction|StartRoll)
    (elif (Variables|Default|GetbNextCombo)
      (Variables|Default|SetbNextCombo false)
      (bind _result (Math|Integer|IncrementInt (Variables|Default|GetComboCount))
        (:%20%20
          (switch int _result
            (:1
              (Animation|PlayAnimMontage "/Game/Characters/Paladin/Animations/sword_and_shield_slash2_Montage.sword_and_shield_slash2_Montage" 1.75 "None"))
            (:2
              (Animation|PlayAnimMontage "/Game/Characters/Paladin/Animations/sword_and_shield_slash3_Montage.sword_and_shield_slash3_Montage" 2.0 "None"))))))))

(event Custom|OnCollision
  ;[1 1 1] On/Off Collision
  (Collision|SetCollisionEnabled (Variables|Default|GetSwordCollision) "QueryAndPhysics"))

(event Custom|OffCollision
  ;[1 1 1] On/Off Collision
  (Collision|SetCollisionEnabled (Variables|Default|GetSwordCollision) "NoCollision")
  (Utilities|Array|Clear (Variables|Default|GetHittedActors)))

(event Custom|EndRoll
  ;[1 1 1] 구르기
  (CallFunction|EndAttack))

(event Custom|StartSpectator
  ;[1 1 1] 구르기
  (Collision|SetCollisionProfileName (Variables|Collision|GetCapsuleComponent) "Spectator" true :!class /Script/Engine.PrimitiveComponent))

(event Custom|EndSpectator
  ;[1 1 1] 구르기
  (Collision|SetCollisionProfileName (Variables|Collision|GetCapsuleComponent) "Pawn" true :!class /Script/Engine.PrimitiveComponent))

(event Custom|StartRoll
  ;[1 1 1] 구르기
  (CallFunction|ForceRotationbyLastInput)
  (bind _output_get (Variables|Default|SetRollStart (Transformation|GetActorLocation)))
  (Variables|Default|SetRollEnd (+ _output_get (* (Transformation|GetActorForwardVector) 3.5e+02)))
  (Animation|PlayAnimMontage "/Game/Characters/Paladin/Animations/Sprinting_Forward_Roll_Montage.Sprinting_Forward_Roll_Montage" 1.25 "None")
  (CallFunction|OffCollision)
  (Components|Timeline|SetPlayRate (Variables|Default|GetRollTimeline) 1.75)
  (bind _output (Timeline|RollTimeline PlayFromStart)
    (:Update
      (Transformation|SetActorLocation (Math|Vector|Lerp(Vector) (Variables|Default|GetRollStart) (Variables|Default|GetRollEnd) _output) true false))))

(event EventBeginPlay
  ;[1 1 1] 비긴플레이 (카메라 세팅)
  (Game|Player|SetViewTargetwithBlend (Game|GetPlayerController 0) (Variables|Default|GetCamera) 0.0 "VTBlend_Linear" 0.0 false)
  (Collision|SetCollisionEnabled (Variables|Default|GetSwordCollision) "NoCollision")
  (bind _returnvalue (Rendering|Material|CreateDynamicMaterialInstance "/Game/Characters/Paladin/Paladin_MAT_Inst.Paladin_MAT_Inst" "None" :!class /Script/Engine.KismetMaterialLibrary))
  (bind _output_get (Variables|Default|SetDynamicMaterial _returnvalue))
  (Rendering|Material|SetMaterial (Variables|Character|GetMesh) 0 _output_get)
  (bind _asbp_game_instance (Utilities|Casting|CastToBP_GameInstance (Game|GetGameInstance)))
  (bind _output_get_2 (Variables|Default|SetGameInstance _asbp_game_instance))
  (Default|ShowPlayerStatus _output_get_2 true)
  (Variables|Default|SetCurrentHP (Variables|Default|GetMaxHP)))

(event Game|Damage|EventAnyDamage
  (params (Damage :type Float%20%28single-precision%29) (DamageType :type Damage%20Type%20Object%20Reference) (InstigatedBy :type Controller%20Object%20Reference) (DamageCauser :type Actor%20Object%20Reference))
  ;[1 1 1] Hitted
  (if (not (Variables|Default|GetbDead))
    (CallFunction|ChangeHitColor)
    (bind _output_get (Variables|Default|SetCurrentHP (- (Variables|Default|GetCurrentHP) Damage)))
    (if (<= _output_get 0.0)
      (Animation|PlayAnimMontage "/Game/Characters/Paladin/Animations/sword_and_shield_death__2__Montage.sword_and_shield_death__2__Montage" 1.0 "None")
      (Variables|Default|SetbDead true)
      (Input|DisableInput 0))))

(event Input|AxisEvents|InputAxisMoveRight
  (params (AxisValue :type Float%20%28single-precision%29))
  ;[1 1 1] 이동
  (CallFunction|IsLastInput AxisValue)
  (if (not (Variables|Default|GetbRolling))
    (if (not (Variables|Default|GetbAttacking))
      (Pawn|Input|AddMovementInput "0,1.000000, 0" AxisValue false))))

(event Input|MouseEvents|LeftMouseButton
  (params (Key :type Key%20Structure :default "None"))
  ;[1 1 1] 공격
  (:Pressed
    (CallFunction|ForceRotationbyLastInput)
    (if (not (Variables|Default|GetbRolling))
      (if (Variables|Default|GetbAttacking)
        (Variables|Default|SetbNextCombo true)
        (else
          (Variables|Default|SetbAttacking true)
          (Animation|PlayAnimMontage "/Game/Characters/Paladin/Animations/sword_and_shield_slash1_Montage.sword_and_shield_slash1_Montage" 1.25 "None"))))))

(event Input|KeyboardEvents|SpaceBar
  (params (Key :type Key%20Structure :default "None"))
  ;[1 1 1] 점프
  (:Pressed
    (if (not (Variables|Default|GetbRolling))
      (if (not (Variables|Default|GetbAttacking))
        (if (not (AI|Components|NavMovement|IsFalling (Variables|Character|GetCharacterMovement)))
          (Audio|PlaySoundatLocation "/Game/Sounds/Jump.Jump" (Transformation|GetActorLocation) "0, 0, 0" 5.0 1.0 0.0 0 0 0)
          (Character|Jump)))))
  (:Released
    (Character|StopJumping)))

(event Input|KeyboardEvents|K
  (params (Key :type Key%20Structure :default "None"))
  ;[1 0 0] Cheat
  (:Pressed
    (bind _outactors (Actor|GetAllActorsOfClass "/Script/Engine.Character"))
    (for _array_element _outactors
      (Utilities|Casting|CastToBP_Player _array_element
        (:CastFailed
          (Game|Damage|ApplyDamage _array_element 999.0 0 self))))))

(event Input|KeyboardEvents|F10
  (params (Key :type Key%20Structure :default "None"))
  (bind _returnvalue (Game|GetPlayerController 0))
  ;[1 1 1] 일시중지 메뉴 호출
  (:Pressed
    (bind _asbp_game_mode_kill_boss (Utilities|Casting|CastToBP_GameMode_KillBoss (Game|GetGameMode)))
    (if (not (Utilities|Enum|Equal(Enum) (Widget|GetVisibility (Variables|/Game/Blueprints/Game/BP_GameMode_KillBoss.BP_GameMode_KillBoss_C|GetStageClearWidget _asbp_game_mode_kill_boss)) "Visible"))
      (if (not (Utilities|Enum|Equal(Enum) (Widget|GetVisibility (Variables|/Game/Blueprints/Game/BP_GameMode_KillBoss.BP_GameMode_KillBoss_C|GetGameOverWidget _asbp_game_mode_kill_boss)) "Visible"))
        (Widget|SetVisibility (Variables|/Game/Blueprints/Game/BP_GameMode_KillBoss.BP_GameMode_KillBoss_C|GetPauseWidget _asbp_game_mode_kill_boss) "Visible")
        (Variables|/Script/Engine.PlayerController|SetbShowMouseCursor _returnvalue true)
        (Input|SetInputModeUIOnly _returnvalue 0 "DoNotLock")
        (Game|SetGamePaused true)))))

(event Input|KeyboardEvents|L
  (params (Key :type Key%20Structure :default "None"))
  ;[1 0 0] Cheat
  (:Pressed
    (bind _outactors (Actor|GetAllActorsOfClass "/Script/Engine.Character"))
    (for _array_element _outactors
      (Utilities|Casting|CastToBP_Player _array_element)
      (Game|Damage|ApplyDamage _array_element 999.0 0 self))))

(event Input|KeyboardEvents|LeftShift
  (params (Key :type Key%20Structure :default "None"))
  ;[1 1 1] 구르기
  (:Pressed
    (if (not (Variables|Default|GetbRolling))
      (Variables|Default|SetbRolling true)
      (if (not (Variables|Default|GetbAttacking))
        (CallFunction|StartRoll)))))

(event Input|KeyboardEvents|J
  (params (Key :type Key%20Structure :default "None"))
  ;[1 0 0] Cheat
  (:Pressed
    (Transformation|SetActorLocation "2200.000000,-550.000000,2550.000000" false false)))

(fn ConstructionScript)

(fn IsOverlappedBody
  (params (OtherComp :type Actor%20Component%20Object%20Reference))
  (bind _componenttags (Variables|/Script/Engine.ActorComponent|GetComponentTags OtherComp))
  (bind _output (Utilities|Array|Get(acopy) _componenttags))
  (if (> (Utilities|Array|Length _componenttags) 0)
    (return (or (Utilities|Name|Equal(Name) _output "Body") (Utilities|Name|Equal(Name) _output "ItemBox")))
    (else
      (return false))))

(fn OnRepCurrentHP
  (Default|UpdateHealth (Variables|/Game/Blueprints/Game/BP_GameInstance.BP_GameInstance_C|GetHudWidget (Variables|Default|GetGameInstance)) (Variables|Default|GetCurrentHP) (Variables|Default|GetMaxHP)))

(fn IsLastInput
  (params (Axis :type Float%20%28single-precision%29))
  (if (< Axis 0.0)
    (Variables|Default|SetbRight false)
    (elif (> Axis 0.0)
      (Variables|Default|SetbRight true))))

(fn ForceRotationbyLastInput
  (if (Variables|Default|GetbRight)
    (Transformation|SetActorRotation "0,90.000000, 0")
    (else
      (Transformation|SetActorRotation "0,-90.000000, 0"))))

(fn IsNotMultiHitted
  (LocalVariables|SetEverHittedActorNumbers (Utilities|Array|Length (Variables|Default|GetHittedActors)))
  (Utilities|Array|AddUnique (Variables|Default|GetHittedActors) (Variables|Default|GetOtherActor))
  (return (< (LocalVariables|GetEverHittedActorNumbers) (Utilities|Array|Length (Variables|Default|GetHittedActors)))))